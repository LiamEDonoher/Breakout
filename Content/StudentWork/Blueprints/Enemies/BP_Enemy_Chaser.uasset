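; Chaser enemy that pursues a target player and fires projectiles, with Move and Attack events and a construction script deferring to its parent.
; Move runs AI MoveTo toward TargetPlayer and zeroes that player's rotation afterwards; its validity check branches to nothing.
; Attack plays a fire sound and spawns BP_Enemy_Projectile at FirePoint with random X/Z jitter and a hard-coded Y.
; The spawned projectile is stored in ShootTimer, despite the variable's name.
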(event `self.Move`
  (bind _targetplayer (`self.TargetPlayer`))
  ;[1 0.003396 0] Moving
  (`/Engine/EditorBlueprintResources/StandardMacros.IsValid` _targetplayer
    (:`Is Valid`
      _)
    (:`Is Not Valid`
      _))
  (`|AIMoveTo` self (0.0 0.0 0.0) _targetplayer
    (:`then`
      (`self.K2_SetActorRotation` :`self` (`self.TargetPlayer`)))))

(event `self.Attack`
  (bind _returnvalue (`KismetMathLibrary.RandomFloatInRange` -20.0 20.0))
  (bind _firepoint (`self.FirePoint`))
  (bind (_returnvalue_x _returnvalue_y _returnvalue_z) (`KismetMathLibrary.BreakVector` (`SceneComponent.K2_GetComponentLocation` _firepoint)))
  ;[1 0.003396 0] Attacking
  (`GameplayStatics.PlaySoundAtLocation` "/Game/StudentWork/Sounds/AUD_DemEnf_Fire.AUD_DemEnf_Fire" (`SceneComponent.K2_GetComponentLocation` (`self.FirePoint`)) (struct) 1.0 1.0 0.0 null null null null)
  (bind _returnvalue_2 (`|SpawnActorFromClass` "/Game/StudentWork/Blueprints/Projectiles/BP_Enemy_Projectile.BP_Enemy_Projectile_C" (`KismetMathLibrary.MakeTransform` (`KismetMathLibrary.MakeVector` (+ _returnvalue_x _returnvalue) -631.256587 (+ _returnvalue_z _returnvalue)) (`SceneComponent.K2_GetComponentRotation` _firepoint)) "Undefined" "MultiplyWithRoot" null null))
  (set `self.ShootTimer` _returnvalue_2))

(fn `UserConstructionScript`
  (`parent.UserConstructionScript`))